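; Effects manager component for ACF characters that adds hit feedback and footstep effects on top of its parent class.
; On damage impacts involving the local player, it shows a damage text widget for nonzero damage and plays a world camera shake and force feedback at the impact point.
; Footstep triggers map the foot to a bone, fire the footstep FX, and play any per-foot impact effect at that bone's location.
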(event EventBeginPlay
  (|CallParentFunction))

(event EventTick
  (params (DeltaSeconds :type Float%20%28single-precision%29)))

(event EventOnDamageImpactReceived
  (params (damageEvent :type ACF%20Damage%20Event%20Structure%20%28by%20ref%29))
  (|CallParentFunction damageEvent)
  (CallFunction|SpawnDamageWidget damageEvent))

(fn SpawnDamageWidget
  (params (ACFDamageEvent :type ACF%20Damage%20Event%20Structure%20%28by%20ref%29))
  (bind _returnvalue (Class|ACFFunctionLibrary|DoesDamageInvolveLocalPlayer ACFDamageEvent))
  (if _returnvalue
    (CallFunction|SpawnWidget ACFDamageEvent)))

(fn TriggerFootstep
  (params (Feet :type EFeets%20Enum :default "NewEnumerator0"))
  (bind _feetbonenames (Variables|ACF|GetFeetBoneNames))
  (bind _characterowner (Variables|Default|GetCharacterOwner))
  (bind _effectsbyfoot (Variables|ACF|GetEffectsByFoot))
  (bind _value (Utilities|Map|Find _feetbonenames Feet))
  (bind (_value_2 _returnvalue) (Utilities|Map|Find _effectsbyfoot Feet))
  (Class|ACFEffectsManagerComponent|TriggerFootstepFX _value)
  (if _returnvalue
    (Class|ACFFunctionLibrary|PlayImpactEffect _value_2 (Transformation|GetSocketLocation (Variables|/Script/Engine.Character|GetMesh _characterowner) _value) _characterowner)))

(fn SpawnDamageText
  (params (ReceivedDamage :type ACF%20Damage%20Event%20Structure))
  (if (!= (.FinalDamage (Utilities|Struct|BreakACFDamageEvent ReceivedDamage)) 0.0)
    (bind _returnvalue (UserInterface|CreateWidget (Variables|ACF|GetDamageWidget) (Game|GetPlayerController 0)))
    (Utilities|IsValid _returnvalue
      (:Is%20Valid
        (UserInterface|Viewport|AddtoViewport _returnvalue 0)
        (Default|SetupDamageText _returnvalue ReceivedDamage)))))

(fn SpawnWidget
  (params (InputPin :type ACF%20Damage%20Event%20Structure%20%28by%20ref%29))
  (bind _hitresult (Utilities|Struct|BreakACFDamageEvent InputPin))
  (bind _impactpoint (Collision|BreakHitResult _hitresult))
  (CallFunction|SpawnDamageText InputPin)
  (Camera|PlayWorldCameraShake "/Game/RPG/Camera/CinematicCamera/Shakes/ACFHitCameraShakeBP.ACFHitCameraShakeBP_C" _impactpoint 0.0 5e+05)
  (ForceFeedback|SpawnForceFeedbackatLocation (Variables|ACF|GetOnHitRumble) _impactpoint "0, 0, 0" false 1.0 0.0 0))