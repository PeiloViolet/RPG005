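; Blueprint function library for the RPG module, holding a single geometry helper, GetsPointOnCircle.
; It takes a center, radius and angle in degrees, converts the angle to radians and uses cosine and sine to return a point on a horizontal circle in the XY plane.
; The returned point keeps the center's Z height.
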(fn GetsPointonCircle
  (params (CenterOfCircle :type Vector) (Radius :type Float%20%28double-precision%29) (Angle :type Float%20%28double-precision%29))
  (bind (_x _y _z) (Math|Vector|BreakVector CenterOfCircle))
  (bind _returnvalue (Math|Float|MultiplybyPi Angle))
  (bind _returnvalue_2 (/ _returnvalue 1.8e+02))
  (return (Math|Vector|MakeVector (+ _x (* Radius (Math|Trig|Cos(Radians) _returnvalue_2))) (+ _y (* (Math|Trig|Sin(Radians) _returnvalue_2) Radius)) _z)))