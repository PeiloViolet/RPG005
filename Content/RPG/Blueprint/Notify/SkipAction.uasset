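; SkipAction is an animation notify state for ALS characters that, as wired, only prints debug information.
; On notify begin it casts the mesh's owning actor to ALSCharacter and prints the current montage's name and active section.
; A networked montage call that would jump to a straight sword combo section is left disconnected, and the tick handler is empty.
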(fn ReceivedNotifyTick
  (params (MeshComp :type Skeletal%20Mesh%20Component%20Object%20Reference) (Animation :type Anim%20Sequence%20Base%20Object%20Reference) (FrameDeltaTime :type Float%20%28single-precision%29) (EventReference :type Anim%20Notify%20Event%20Reference%20Structure%20%28by%20ref%29)))

(fn ReceivedNotifyBegin
  (params (MeshComp :type Skeletal%20Mesh%20Component%20Object%20Reference) (Animation :type Anim%20Sequence%20Base%20Object%20Reference) (TotalDuration :type Float%20%28single-precision%29) (EventReference :type Anim%20Notify%20Event%20Reference%20Structure%20%28by%20ref%29))
  (bind _returnvalue (Components|SkeletalMesh|GetAnimInstance MeshComp))
  (bind _returnvalue_2 (Class|AnimInstance|GetOwningActor _returnvalue))
  (Utilities|IsValid _returnvalue_2
    (:Is%20Valid
      (bind _asalscharacter (Utilities|Casting|CastToALSCharacter _returnvalue_2))
      (Development|PrintString 0 (Utilities|GetDisplayName (Animation|GetCurrentMontage _asalscharacter :!class /Script/Engine.Character)))
      (Development|PrintString 0 (Utilities|String|ToString(Name) (Animation|Montage|MontageGetCurrentSection _returnvalue (Animation|GetCurrentMontage _asalscharacter :!class /Script/Engine.Character))))
      (return true))))