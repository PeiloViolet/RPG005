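; RPG game instance that provides entry points for starting a new game and loading the default save.
; NewGame clears the Restarted flag, marks a new game on the ALS Load and Save subsystem, then opens the default level by name.
; LoadDefaultSave asks that subsystem to load the game world from the stored slot name, which a getter also exposes.
; The OnGameLoaded handler is an empty stub.
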(fn NewGame
  (Variables|Default|SetRestarted false)
  (Class|ALSLoadandSaveSubsystem|SetNewGame (Subsystems|GetALSLoadandSaveSubsystem) true)
  (Game|OpenLevel(byName) (Variables|Default|GetDefaultLevel)))

(fn LoadDefaultSave
  (Class|ALSLoadandSaveSubsystem|LoadGameWorld (Subsystems|GetALSLoadandSaveSubsystem) (Variables|Default|GetSlot%20Name) (EventDispatchers|CreateEvent :!event OnGameLoaded)))

(fn GetDefaultSlotname
  (return (Variables|Default|GetSlot%20Name)))

(fn OnGameLoaded
  (params (Success :type Boolean)))