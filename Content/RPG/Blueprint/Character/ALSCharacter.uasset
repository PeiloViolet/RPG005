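; RPG character built on ALS, with targeting widgets, shooting, abilities and stamina-limited sprint.
; BeginPlay links locomotion and overlay anim layers, then initializes health widget, shooting and abilities.
; Overlay mode drives held-prop sockets, linked layers and mantling settings; combat-type handler updates camera and strafe, but its binding here is unwired.
; Debug helpers print capsule distance to the target every tick and toggle slow motion through server-to-multicast events.
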(event OnStatisiticReachesZero(StatisticsComp)
  (params (Stat :type Gameplay%20Tag%20Structure))
  (if (== Stat "(TagName=\"RPG.Statistic.Stamina\")")
    (Class|RPGCharacter|StopSprint)))

(event Custom|服务器时间膨胀
  (CallFunction|多播时间膨胀))

(event Custom|多播时间膨胀
  (Utilities|FlowControl|FlipFlop
    (:A
      (Utilities|Time|SetGlobalTimeDilation 0.1))
    (:B
      (Utilities|Time|SetGlobalTimeDilation 1.0))))

(event EventBeginPlay
  (|CallParentFunction)
  (|初始化))

(event EventTick
  (params (DeltaSeconds :type Float%20%28single-precision%29))
  (bind _output_get (Variables|Default|SetDelta%20Seconds DeltaSeconds))
  (|CallParentFunction _output_get)
  (|Test))

(event Input|ActionEvents|InputActionTest
  (params (Key :type Key%20Structure :default "None")))

(event Input|ActionEvents|InputAction时间膨胀
  (params (Key :type Key%20Structure :default "None"))
  (:Pressed
    (CallFunction|服务器时间膨胀)))

(event Input|ActionEvents|InputActionTest2
  (params (Key :type Key%20Structure :default "None")))

(fn ConstructionScript)

(fn RefreshOverlayObject
  (|SwitchGameplayTag (Variables|Default|GetOverlayMode)
    (:Default
      (Overlay|ClearOverlayObject))
    (:Als.OverlayMode.M4
      (Overlay|AttachOverlayObject 0 0 0 "M4" false))
    (:Als.OverlayMode.PistolOneHanded
      (Overlay|AttachOverlayObject 0 0 0 "M9" false :!label _label))
    (:Als.OverlayMode.PistolTwoHanded
      (goto _label))
    (:Als.OverlayMode.Bow
      (Overlay|AttachOverlayObject 0 0 0 "Bow" true))
    (:Als.OverlayMode.Torch
      (Overlay|AttachOverlayObject 0 0 0 "Torch" true))
    (:Als.OverlayMode.Binoculars
      (Overlay|AttachOverlayObject 0 0 0 "Binoculars" false))
    (:Als.OverlayMode.Box
      (Overlay|AttachOverlayObject 0 0 0 "Box" false))
    (:Als.OverlayMode.Barrel
      (Overlay|AttachOverlayObject 0 0 0 "Barrel" true))))

(fn ClearOverlayObject
  (Components|StaticMesh|SetStaticMesh (Variables|Default|GetOverlayStaticMesh) 0)
  (Class|SkinnedMeshComponent|SetSkeletalMesh (Variables|Default|GetOverlaySkeletalMesh) 0 true)
  (Class|SkeletalMeshComponent|SetAnimClass (Variables|Default|GetOverlaySkeletalMesh)))

(fn RefreshOverlayLinkedAnimationLayer
  (bind _mesh (Variables|Character|GetMesh))
  (LocalVariables|SetOverlayAnimationInstanceClass (.Value (Utilities|Map|Find (Variables|Settings|AlsCharacter|GetOverlayAnimationInstanceClasses) (Variables|Default|GetOverlayMode))))
  (bind _overlayanimationinstanceclass (LocalVariables|GetOverlayAnimationInstanceClass)
    (:then
      (Components|SkeletalMesh|AnimationBlueprintLinking|LinkAnimClassLayers _mesh _overlayanimationinstanceclass))
    (:else
      (Components|SkeletalMesh|AnimationBlueprintLinking|LinkAnimClassLayers _mesh "/Game/RPG/Blueprint/Character/AnimationInstances/Overlays/AB_Als_Default.AB_Als_Default_C"))))

(fn AttachOverlayObject
  (params (NewStaticMesh :type Static%20Mesh%20Object%20Reference) (NewSkeletalMesh :type Skeletal%20Mesh%20Object%20Reference) (NewAnimationClass :type Anim%20Instance%20Class%20Reference) (SocketName :type Name) (bUseLeftGunBone :type Boolean))
  (LocalVariables|SetResultSocketName (select (Variables|Settings|AlsCharacter|GetbUseGunBoneForOverlayObjects) (select bUseLeftGunBone "None" "None") SocketName))
  (Utilities|FlowControl|Sequence
    (:then_0
      (Components|StaticMesh|SetStaticMesh (Variables|Default|GetOverlayStaticMesh) NewStaticMesh)
      (Transformation|AttachComponentToComponent (Variables|Default|GetOverlayStaticMesh) (Variables|Character|GetMesh) (LocalVariables|GetResultSocketName) "SnapToTarget" "SnapToTarget" "SnapToTarget" true))
    (:then_1
      (Class|SkinnedMeshComponent|SetSkeletalMesh (Variables|Default|GetOverlaySkeletalMesh) NewSkeletalMesh true)
      (Class|SkeletalMeshComponent|SetAnimClass (Variables|Default|GetOverlaySkeletalMesh) NewAnimationClass)
      (Transformation|AttachComponentToComponent (Variables|Default|GetOverlaySkeletalMesh) (Variables|Character|GetMesh) (LocalVariables|GetResultSocketName) "SnapToTarget" "SnapToTarget" "SnapToTarget" true))))

(fn SelectMantlingSettings
  (params (MantlingType :type EAlsMantlingType%20Enum :default "High"))
  (switch Utilities|FlowControl|Switch|SwitchonEAlsMantlingType MantlingType
    (:High
      _)
    (:Low
      (|SwitchGameplayTag (Variables|Default|GetOverlayMode)
        (:Default
          (return "/Game/RPG/Data/Character/Mantle/MS_Low.MS_Low"))
        (:Als.OverlayMode.Injured
          _)
        (:Als.OverlayMode.HandsTied
          (return "/Game/RPG/Data/Character/Mantle/MS_Low_BothHands.MS_Low_BothHands"))
        (:Als.OverlayMode.M4
          (return "/Game/RPG/Data/Character/Mantle/MS_Low_Right.MS_Low_Right"))
        (:Als.OverlayMode.PistolOneHanded
          (return "/Game/RPG/Data/Character/Mantle/MS_Low_Right.MS_Low_Right"))
        (:Als.OverlayMode.PistolTwoHanded
          (return "/Game/RPG/Data/Character/Mantle/MS_Low_Right.MS_Low_Right"))
        (:Als.OverlayMode.Bow
          _)
        (:Als.OverlayMode.Torch
          _)
        (:Als.OverlayMode.Binoculars
          (return "/Game/RPG/Data/Character/Mantle/MS_Low_Right.MS_Low_Right"))
        (:Als.OverlayMode.Box
          (return "/Game/RPG/Data/Character/Mantle/MS_Low_Box.MS_Low_Box"))
        (:Als.OverlayMode.Barrel
          _))
      (return "/Game/RPG/Data/Character/Mantle/MS_Low_Left.MS_Low_Left"))
    (:InAir
      _))
  (return "/Game/RPG/Data/Character/Mantle/MS_High.MS_High"))

(fn RefreshBaseLocomotionLinkedAnimationLayer
  (bind _mesh (Variables|Character|GetMesh))
  (LocalVariables|SetBaseLayerAnimationInstanceClass (.Value (Utilities|Map|Find (Variables|Settings|AlsCharacter|GetLocomotionAnimationInstanceClasses) (Variables|Default|GetBaseLayerMode))))
  (bind _baselayeranimationinstanceclass (LocalVariables|GetBaseLayerAnimationInstanceClass)
    (:then
      (Components|SkeletalMesh|AnimationBlueprintLinking|LinkAnimClassLayers _mesh _baselayeranimationinstanceclass))
    (:else
      (Components|SkeletalMesh|AnimationBlueprintLinking|LinkAnimClassLayers _mesh "/Game/RPG/Blueprint/Character/AnimationInstances/ALS_BaseLayer/AB_ALS_BaseLayer.AB_ALS_BaseLayer_C"))))

(fn GetsTargeted
  (params (point :type ATS%20Target%20Point%20Component%20Object%20Reference))
  (bind _healthwidget (Variables|Default|GetHealthWidget))
  (bind _returnvalue (UserInterface|GetUserWidgetObject _healthwidget))
  (Development|SetHiddeninGame (Variables|Default|GetTargetedWidget) false true)
  (Development|SetHiddeninGame _healthwidget false true)
  (Utilities|IsValid _returnvalue
    (:Is%20Valid
      (Widget|Transform|SetRenderScale _returnvalue (Math|Vector2D|MakeVector2D 0.5 0.5))
      (return))))

(fn LoseTargeted
  (Development|SetHiddeninGame (Variables|Default|GetTargetedWidget) true true)
  (Development|SetHiddeninGame (Variables|Default|GetHealthWidget) true true)
  (return))

(fn RefreshHealthWidget
  (bind _ashealth_widget (Utilities|Casting|CastToHealthWidget (UserInterface|GetWidget (Variables|Default|GetHealthWidget))))
  (Default|初始化控件 _ashealth_widget self))

(fn SetStrafe
  (Class|ACFCharacter|SetStrafeMovement (CallFunction|ShouldStrafe)))

(fn ShouldStrafe
  (bind _returnvalue (Pawn|GetController))
  (bind _returnvalue_2 (Actor|GetComponentbyClass _returnvalue "/Script/TargetingSystem.ATSTargetingComponent"))
  (Utilities|IsValid _returnvalue
    (:Is%20Valid
      (Utilities|IsValid _returnvalue_2
        (:Is%20Valid
          (return (Math|Boolean|ORBoolean false (Class|ACFCharacter|IsRanged) (Class|ATSTargetingComponent|IsTargetingEnabled _returnvalue_2))))))))

(event Custom|HandleCombatTypeCHanged
  (params (CombatType :type ECombatType%20Enum :default "EUnarmed"))
  (switch Utilities|FlowControl|Switch|SwitchonECombatType CombatType
    (:EUnarmed
      (Class|CCMCameraFunctionLibrary|StopCameraEvent "Equip"))
    (:EMelee
      (Class|CCMCameraFunctionLibrary|TriggerCameraEvent "Equip" :!label _label))
    (:ERanged
      (goto _label)))
  (CallFunction|SetStrafe))