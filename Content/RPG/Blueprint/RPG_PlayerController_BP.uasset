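; RPG player controller Blueprint that sets up local input and carries a debug team switch.
; On BeginPlay, the local controller switches to game-only input and adds the default Enhanced Input mapping context.
; A Test input action sets the combat team to TestTeam and prints a switch-to-team-4 message.
; An unconnected branch would load the default save through the RPG game instance, but it never runs.
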(event EventTick
  (params (DeltaSeconds :type Float%20%28single-precision%29))
  (|CallParentFunction DeltaSeconds))

(event EventBeginPlay
  (if (Pawn|IsLocalController)
    (Input|SetInputModeGameOnly self)
    (Input|AddMappingContext (PlayerController|LocalPlayerSubsystems|GetEnhancedInputLocalPlayerSubsystem) "/Game/RPG/Data/Input/IMC_Default.IMC_Default" 0 "(bIgnoreAllPressedKeysUntilRelease=True,bForceImmediately=False)")))

(event Input|ActionEvents|InputActionTest
  (params (Key :type Key%20Structure))
  (:Pressed
    (Class|ACFPlayerController|SetCombatTeam (Variables|Default|GetTestTeam))
    (Development|PrintString "切换到队伍4")))

(fn ConstructionScript)