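; AI_Base_BP is an RPG enemy AI base Blueprint that shows targeting feedback through widget components.
; On BeginPlay it casts the health component's widget to HealthWidget and initializes it with itself as the owner.
; Target acquired and lost events reveal or hide both the target marker and health bar, propagating visibility to child components.
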(event EventBeginPlay
  (CallFunction|RefreshHealthWidget))

(event EventOnTargetLosed
  (CallFunction|LoseTargeted))

(event EventOnTargetAcquired
  (params (point :type ATS%20Target%20Point%20Component%20Object%20Reference))
  (CallFunction|GetsTargeted point))

(fn ConstructionScript)

(fn GetsTargeted
  (params (InputObject :type ATS%20Target%20Point%20Component%20Object%20Reference))
  (Development|SetHiddeninGame (Variables|Default|GetTargetedWidget) false true)
  (Development|SetHiddeninGame (Variables|Default|GetHealthWidget) false true))

(fn LoseTargeted
  (Development|SetHiddeninGame (Variables|Default|GetTargetedWidget) true true)
  (Development|SetHiddeninGame (Variables|Default|GetHealthWidget) true true))

(fn RefreshHealthWidget
  (bind _ashealth_widget (Utilities|Casting|CastToHealthWidget (UserInterface|GetWidget (Variables|Default|GetHealthWidget))))
  (Default|初始化控件 _ashealth_widget self))