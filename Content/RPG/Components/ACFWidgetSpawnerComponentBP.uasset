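; Widget spawner component for ACF that shows a modal UI widget, with events named for routing to the owning client.
; Spawning creates and stores the widget, switches to UI-only input with cursor, blocks look input, sets pause from PauseGame and stops the local ACF character's movement.
; Removing the stored or a given widget goes through InternalRemoveWidget, which restores game input, hides the cursor and unpauses.
; Both paths act on player controller 0.
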(event Custom|RemoveCurrentWidget
  (CallFunction|ClientRemoveCurrentWidget))

(event Custom|ClientSpawnWidget
  (params (Class :type User%20Widget%20Class%20Reference))
  (bind _returnvalue (Class|ACFFunctionLibrary|GetLocalACFPlayerCharacter))
  (bind _returnvalue_2 (UserInterface|CreateWidget Class (Game|GetPlayerController 0)))
  (bind _output_get (Variables|Default|SetWidgetShown _returnvalue_2))
  (UserInterface|Viewport|AddtoViewport _output_get 2)
  (Input|SetInputModeUIOnly (Game|GetPlayerController 0) (Variables|Default|GetWidgetShown) "LockAlways")
  (Variables|/Script/Engine.PlayerController|SetbShowMouseCursor (Game|GetPlayerController 0) true)
  (Input|SetIgnoreLookInput (Game|GetPlayerController 0) true)
  (Game|SetGamePaused (Variables|Default|GetPause%20Game))
  (Utilities|IsValid _returnvalue
    (:Is%20Valid
      (Components|Movement|StopMovementImmediately (Variables|/Script/Engine.Character|GetCharacterMovement _returnvalue)))))

(event Custom|RemoveWidget
  (params (Widget :type Widget%20Object%20Reference))
  (CallFunction|InternalRemoveWidget Widget))

(event Custom|SpawnWidgetToOwningClient
  (params (Class :type User%20Widget%20Class%20Reference))
  (CallFunction|ClientSpawnWidget Class))

(event Custom|ClientRemoveCurrentWidget
  (CallFunction|InternalRemoveWidget (Variables|Default|GetWidgetShown)))

(event EventBeginPlay)

(event EventTick
  (params (DeltaSeconds :type Float%20%28single-precision%29)))

(fn InternalRemoveWidget
  (params (Target :type Widget%20Object%20Reference))
  (bind _returnvalue (Game|GetPlayerController 0))
  (Widget|RemovefromParent Target)
  (Input|SetInputModeGameOnly (Game|GetPlayerController 0))
  (Variables|/Script/Engine.PlayerController|SetbShowMouseCursor _returnvalue false)
  (Game|SetGamePaused false)
  (Input|SetInputModeGameOnly _returnvalue)
  (Input|SetIgnoreLookInput (Game|GetPlayerController 0) false))